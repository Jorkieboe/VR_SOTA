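; Player character that walks, looks around, interacts with actors and answers NPC dialog with a left or right choice.
; Either trigger runs a short horizontal line trace along the actor's forward vector, stores a hit VRInteractionBPI actor and sends it TriggerPressedMessage.
; Toggleondialog shows the dialog widget and enables choices.
; A choice closes the widget and sets Right and Next on the stored actor if it is an NPCCharacter.
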(event Custom|Toggle%20on%20dialog
  (bind _returnvalue (UserInterface|CreateWidget "/Game/VR/blueprints/dialogwidget.dialogwidget_C"))
  (Variables|Default|SetDialogWidget _returnvalue)
  (UserInterface|Viewport|AddtoViewport _returnvalue 0)
  (Variables|Default|SetCanNext true))

(event EventBeginPlay)

(event Collision|EventActorBeginOverlap
  (params (OtherActor :type Actor%20Object%20Reference)))

(event EventTick
  (params (DeltaSeconds :type Float%20%28single-precision%29)))

(event Input|ActionEvents|InputActionTriggerLeft
  (params (Key :type Key%20Structure :default "None"))
  (bind _returnvalue (Transformation|GetActorLocation))
  (:Pressed
    (bind _outhit (Collision|LineTraceByChannel _returnvalue (+ _returnvalue (* (Transformation|GetActorForwardVector) "500.000000,500.000000,0")) "TraceTypeQuery1" false 0 "ForDuration"))
    (if (Utilities|DoesObjectImplementInterface (.hitactor _outhit) "/Game/VRTemplate/Blueprints/VRInteractionBPI.VRInteractionBPI_C")
      (bind _output_get (Variables|Default|SetHitted%20actor (.hitactor _outhit)))
      (Development|PrintString (Utilities|GetDisplayName _output_get))
      (Class|VRInteractionBPI|TriggerPressed(Message) (.hitactor _outhit)))))

(event Input|ActionEvents|InputActionTriggerRight
  (params (Key :type Key%20Structure :default "None"))
  (bind _returnvalue (Transformation|GetActorLocation))
  (:Pressed
    (bind _outhit (Collision|LineTraceByChannel _returnvalue (+ _returnvalue (* (Transformation|GetActorForwardVector) "500.000000,500.000000,0")) "TraceTypeQuery1" false 0 "ForDuration"))
    (if (Utilities|DoesObjectImplementInterface (.hitactor _outhit) "/Game/VRTemplate/Blueprints/VRInteractionBPI.VRInteractionBPI_C")
      (bind _output_get (Variables|Default|SetHitted%20actor (.hitactor _outhit)))
      (Development|PrintString (Utilities|GetDisplayName _output_get))
      (Class|VRInteractionBPI|TriggerPressed(Message) (.hitactor _outhit)))))

(event Input|ActionEvents|InputActionTextOptionLeft
  (params (Key :type Key%20Structure :default "None"))
  (bind _dialogwidget (Variables|Default|GetDialogWidget))
  (:Pressed
    (if (Variables|Default|GetCanNext)
      (Default|Left _dialogwidget)
      (Widget|RemovefromParent _dialogwidget)
      (Variables|Default|SetCanNext false)
      (bind _asnpccharacter (Utilities|Casting|CastToNPCCharacter (Variables|Default|GetHitted%20actor)))
      (Variables|/Game/VR/npcs/NPCCharacter.NPCCharacter_C|SetRight _asnpccharacter false)
      (Variables|/Game/VR/npcs/NPCCharacter.NPCCharacter_C|SetNext _asnpccharacter true))))

(event Input|ActionEvents|InputActionTextOptionRight
  (params (Key :type Key%20Structure :default "None"))
  (bind _dialogwidget (Variables|Default|GetDialogWidget))
  (:Pressed
    (if (Variables|Default|GetCanNext)
      (Default|Right _dialogwidget)
      (Widget|RemovefromParent _dialogwidget)
      (Variables|Default|SetCanNext false)
      (bind _asnpccharacter (Utilities|Casting|CastToNPCCharacter (Variables|Default|GetHitted%20actor)))
      (Variables|/Game/VR/npcs/NPCCharacter.NPCCharacter_C|SetRight _asnpccharacter true)
      (Variables|/Game/VR/npcs/NPCCharacter.NPCCharacter_C|SetNext _asnpccharacter true))))

(event Input|AxisEvents|InputAxisside
  (params (AxisValue :type Float%20%28single-precision%29))
  (Pawn|Input|AddControllerYawInput AxisValue))

(event Input|AxisEvents|InputAxiswalkforwards
  (params (AxisValue :type Float%20%28single-precision%29))
  (Pawn|Input|AddMovementInput (Transformation|GetActorForwardVector) AxisValue false))

(event Input|AxisEvents|InputAxiswalksideways
  (params (AxisValue :type Float%20%28single-precision%29))
  (Pawn|Input|AddMovementInput (Transformation|GetActorRightVector) AxisValue false))

(event Input|AxisEvents|InputAxisup
  (params (AxisValue :type Float%20%28single-precision%29))
  (Pawn|Input|AddControllerPitchInput (* AxisValue -1.0)))

(fn ConstructionScript)
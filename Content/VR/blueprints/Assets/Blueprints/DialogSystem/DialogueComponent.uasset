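; Dialogue component that runs conversations through a behavior tree and an on-screen dialog widget.
; BeginPlay spawns a DialogAIController, then flows into the same setup that OnInteract triggers: create the widget, switch to UI-only input with cursor, and run DialogTree.
; The widget is passed to the tree through the blackboard.
; The widget's exit event restores game input, stops the tree and removes the widget.
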(event Custom|onExit_Event_0
  (bind _dialogwidget (Variables|Default|GetDialogWidget))
  (bind _returnvalue (Widget|GetOwningPlayer _dialogwidget))
  (Input|SetInputModeGameOnly _returnvalue)
  (Variables|/Script/Engine.PlayerController|SetbShowMouseCursor _returnvalue false)
  (AI|Logic|StopLogic (Variables|/Script/AIModule.AIController|GetBrainComponent (Variables|Default|GetAIController)) "Dialog Exited")
  (Widget|RemovefromParent (Variables|Default|GetDialogWidget)))

(event EventBeginPlay
  (bind _returnvalue (Game|SpawnActorfromClass "/Game/VR/blueprints/Assets/Blueprints/DialogSystem/DialogAIController.DialogAIController_C" (Math|Transform|MakeTransform "0, 0, 0" "0, 0, 0" "1.000000,1.000000,1.000000") "Undefined" 0 0))
  (Variables|Default|SetAIController _returnvalue)
  (Development|PrintString "doet")
  (bind _returnvalue_2 (UserInterface|CreateWidget "/Game/VR/blueprints/Assets/Blueprints/DialogSystem/DialogWidget.DialogWidget_C" (.AsPlayer%20Controller (Utilities|Casting|CastToPlayerController (stale EventOnInteract Player)))))
  (Development|PrintString "Hello")
  (bind _output_get (Variables|Default|SetDialogWidget _returnvalue_2))
  (EventDispatchers|BindEventtoOnExit _output_get (delegate Custom|onExit_Event_0))
  (UserInterface|Viewport|AddtoViewport _output_get 0)
  (Input|SetInputModeUIOnly (.AsPlayer%20Controller (Utilities|Casting|CastToPlayerController (stale EventOnInteract Player))) _output_get "DoNotLock")
  (Variables|/Script/Engine.PlayerController|SetbShowMouseCursor (.AsPlayer%20Controller (Utilities|Casting|CastToPlayerController (stale EventOnInteract Player))) true)
  (AI|RunBehaviorTree (Variables|Default|GetAIController) (Variables|Default|GetDialogTree))
  (bind _blackboardcomponent (Class|AIController|UseBlackboard (Variables|Default|GetAIController) "/Game/VR/blueprints/Assets/Blueprints/DialogSystem/DialogBlackBoard.DialogBlackBoard"))
  (AI|Components|Blackboard|SetValueasObject _blackboardcomponent (Utilities|Name|MakeLiteralName "DialogWidget") (Variables|Default|GetDialogWidget)))

(event EventOnInteract
  (params (Player :type Object%20Object%20Reference))
  (bind _asplayer_controller (Utilities|Casting|CastToPlayerController Player))
  (bind _returnvalue (UserInterface|CreateWidget "/Game/VR/blueprints/Assets/Blueprints/DialogSystem/DialogWidget.DialogWidget_C" _asplayer_controller))
  (Development|PrintString "Hello")
  (bind _output_get (Variables|Default|SetDialogWidget _returnvalue))
  (EventDispatchers|BindEventtoOnExit _output_get (delegate Custom|onExit_Event_0))
  (UserInterface|Viewport|AddtoViewport _output_get 0)
  (Input|SetInputModeUIOnly _asplayer_controller _output_get "DoNotLock")
  (Variables|/Script/Engine.PlayerController|SetbShowMouseCursor _asplayer_controller true)
  (AI|RunBehaviorTree (Variables|Default|GetAIController) (Variables|Default|GetDialogTree))
  (bind _blackboardcomponent (Class|AIController|UseBlackboard (Variables|Default|GetAIController) "/Game/VR/blueprints/Assets/Blueprints/DialogSystem/DialogBlackBoard.DialogBlackBoard"))
  (AI|Components|Blackboard|SetValueasObject _blackboardcomponent (Utilities|Name|MakeLiteralName "DialogWidget") (Variables|Default|GetDialogWidget)))
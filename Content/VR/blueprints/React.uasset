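; Behavior tree task that runs a two-choice dialogue step between an NPC and the player.
; On execute it shows its text on the NPC's widget, passes left and right options to the player controller, toggles dialogue on and flags responding.
; Each tick it checks the NPC's Next flag, then writes the chosen side to the Right blackboard key, clears responding and finishes successfully.
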(event EventReceiveTickAI
  (params (OwnerController :type AI%20Controller%20Object%20Reference) (ControlledPawn :type Pawn%20Object%20Reference) (DeltaSeconds :type Float%20%28single-precision%29))
  (bind _asnpccharacter (Utilities|Casting|CastToNPCCharacter ControlledPawn))
  (if (Variables|/Game/VR/npcs/NPCCharacter.NPCCharacter_C|GetNext _asnpccharacter)
    (Variables|/Game/VR/npcs/NPCCharacter.NPCCharacter_C|SetNext _asnpccharacter false)
    (Class|BTFunctionLibrary|SetBlackboardValueasBool (Variables|Default|GetRight) (Variables|/Game/VR/npcs/NPCCharacter.NPCCharacter_C|GetRight _asnpccharacter))
    (bind _asbp_player_con (Utilities|Casting|CastToBP_playerCon (Game|GetPlayerController 0)))
    (Variables|/Game/VR/blueprints/BP_playerCon.BP_playerCon_C|SetResponding _asbp_player_con false)
    (AI|BehaviorTree|FinishExecute true)))

(event EventReceiveExecuteAI
  (params (OwnerController :type AI%20Controller%20Object%20Reference) (ControlledPawn :type Pawn%20Object%20Reference))
  (bind _asnpccharacter (Utilities|Casting|CastToNPCCharacter ControlledPawn))
  (Variables|/Game/VR/blueprints/Assets/Blueprints/DialogSystem/newdiawidget.newdiawidget_C|SetText (Variables|/Game/VR/npcs/NPCCharacter.NPCCharacter_C|Getdialogwidget _asnpccharacter) (Variables|Default|GetText))
  (UserInterface|SetWidget (Variables|/Game/VR/npcs/NPCCharacter.NPCCharacter_C|GetWidget _asnpccharacter) (Variables|/Game/VR/npcs/NPCCharacter.NPCCharacter_C|Getdialogwidget _asnpccharacter))
  (bind _asplayer_character (Utilities|Casting|CastToplayerCharacter (Game|GetPlayerCharacter 0)))
  (bind _asbp_player_con (Utilities|Casting|CastToBP_playerCon (Game|GetPlayerController 0)))
  (Variables|/Game/VR/blueprints/BP_playerCon.BP_playerCon_C|SetTextLeft _asbp_player_con (Variables|Default|GetOption%20Left))
  (Variables|/Game/VR/blueprints/BP_playerCon.BP_playerCon_C|SetTextRight _asbp_player_con (Variables|Default|GetOption%20Right))
  (Default|ToggleonDialog _asplayer_character)
  (Variables|/Game/VR/blueprints/BP_playerCon.BP_playerCon_C|SetResponding _asbp_player_con true))
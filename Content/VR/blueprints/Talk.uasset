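; Talk is a behavior tree task that shows one line of NPC dialogue.
; On execute it scans every NPCCharacter, sets the text on those whose DialogID matches NPCId and clears it on all others.
; It then ticks until the controlled NPCCharacter's Next flag is set, resets that flag and finishes successfully, so the tree can advance.
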(event EventReceiveTickAI
  (params (OwnerController :type AI%20Controller%20Object%20Reference) (ControlledPawn :type Pawn%20Object%20Reference) (DeltaSeconds :type Float%20%28single-precision%29))
  (bind _asnpccharacter (Utilities|Casting|CastToNPCCharacter ControlledPawn))
  (if (Variables|/Game/VR/npcs/NPCCharacter.NPCCharacter_C|GetNext _asnpccharacter)
    (Variables|/Game/VR/npcs/NPCCharacter.NPCCharacter_C|SetNext _asnpccharacter false)
    (AI|BehaviorTree|FinishExecute true)))

(event EventReceiveExecuteAI
  (params (OwnerController :type AI%20Controller%20Object%20Reference) (ControlledPawn :type Pawn%20Object%20Reference))
  (bind _outactors (Actor|GetAllActorsOfClass "/Game/VR/npcs/NPCCharacter.NPCCharacter_C"))
  (for _array_element _outactors
    (if (== (Variables|Default|GetNPCId) (Variables|/Game/VR/npcs/NPCCharacter.NPCCharacter_C|GetDialogID _array_element))
      (Default|SetText _array_element (Utilities|Text|ToText(String) (Variables|Default|GetText)))
      (else
        (Default|SetText _array_element)))))
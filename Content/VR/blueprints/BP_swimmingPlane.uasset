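; BP_swimmingPlane is a water trigger that marks when the player is swimming and drives the swimming energy mechanic.
; Its Collision overlaps set the Swimming flag on BP_playerCon for PlayerCharacter or VRPawn, and leaving also resets Energy to full.
; It caches the controller on BeginPlay and calls DecreaseSwimming every Tick, even without overlap, leaving the drain logic to the controller.
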(event OnComponentBeginOverlap(collision)
  (params (OverlappedComponent :type Primitive%20Component%20Object%20Reference) (OtherActor :type Actor%20Object%20Reference) (OtherComp :type Primitive%20Component%20Object%20Reference) (OtherBodyIndex :type Integer) (bFromSweep :type Boolean) (SweepResult :type Hit%20Result%20Structure%20%28by%20ref%29))
  (bind _returnvalue (Utilities|GetClass OtherActor))
  (Development|PrintString "overlap")
  (if (or (== _returnvalue "/Game/VR/blueprints/Assets/Blueprints/playerCharacter.playerCharacter_C") (== _returnvalue "/Game/VRTemplate/Blueprints/VRPawn.VRPawn_C"))
    (bind _asbp_player_con (Utilities|Casting|CastToBP_playerCon (Game|GetPlayerController 0)))
    (Variables|/Game/VR/blueprints/BP_playerCon.BP_playerCon_C|SetSwimming _asbp_player_con true)))

(event OnComponentEndOverlap(collision)
  (params (OverlappedComponent :type Primitive%20Component%20Object%20Reference) (OtherActor :type Actor%20Object%20Reference) (OtherComp :type Primitive%20Component%20Object%20Reference) (OtherBodyIndex :type Integer))
  (bind _returnvalue (Utilities|GetClass OtherActor))
  (if (or (== _returnvalue "/Game/VR/blueprints/Assets/Blueprints/playerCharacter.playerCharacter_C") (== _returnvalue "/Game/VRTemplate/Blueprints/VRPawn.VRPawn_C"))
    (bind _asbp_player_con (Utilities|Casting|CastToBP_playerCon (Game|GetPlayerController 0)))
    (Variables|/Game/VR/blueprints/BP_playerCon.BP_playerCon_C|SetSwimming _asbp_player_con false)
    (Variables|/Game/VR/blueprints/BP_playerCon.BP_playerCon_C|SetEnergy _asbp_player_con 100)))

(event EventBeginPlay
  (bind _asbp_player_con (Utilities|Casting|CastToBP_playerCon (Game|GetPlayerController 0)))
  (Variables|Default|SetAs%20BP%20Player%20Con _asbp_player_con))

(event Collision|EventActorBeginOverlap
  (params (OtherActor :type Actor%20Object%20Reference)))

(event EventTick
  (params (DeltaSeconds :type Float%20%28single-precision%29))
  (Default|DecreaseSwimming (Variables|Default|GetAs%20BP%20Player%20Con)))

(fn ConstructionScript)
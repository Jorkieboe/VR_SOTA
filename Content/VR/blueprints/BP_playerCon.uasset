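; VR player controller that handles swimming stamina, death, level restart and the quest start screen.
; Each Decreaseswimming call drains Energy while swimming, switches to faster-repeating swim sounds as it falls, and at zero disables input and shows DeathScreen.
; Tick requests the sound, throttled by a delay-reset gate.
; Startquest runs once, advancing the VRGameMode quest and briefly showing QuestScreen; the Restart input reopens the Beach level.
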(event Custom|Decrease%20swimming
  (bind _energy (Variables|Default|GetEnergy))
  (if (Variables|Default|GetSwimming)
    (Math|Integer|DecrementInt _energy
      (:%20%20
        (if (< _energy 40)
          (if (< _energy 20)
            (Variables|Default|Setsound%20delay 1.4)
            (Variables|Default|SetSound "/Game/VR/sounds/Swimming3.Swimming3")
            (else
              (Variables|Default|Setsound%20delay 1.7)
              (Variables|Default|SetSound "/Game/VR/sounds/Swimming2.Swimming2")))
          (else
            (Variables|Default|Setsound%20delay 2.0)
            (Variables|Default|SetSound "/Game/VR/sounds/Swimming1.Swimming1")))
        (if (== _energy 0)
          (Input|DisableInput (Game|GetPlayerCharacter 0) self)
          (bind _returnvalue (UserInterface|CreateWidget "/Game/VR/blueprints/DeathScreen.DeathScreen_C"))
          (UserInterface|Viewport|AddtoViewport _returnvalue 0)
          (Variables|Default|SetSwimming false))))))

(event Custom|Start%20quest
  (if (not (Variables|Default|Getquest%20started?))
    (Variables|Default|Setquest%20started? true)
    (bind _asvrgame_mode (Utilities|Casting|CastToVRGameMode (Game|GetGameMode)))
    (Math|Integer|IncrementInt (Variables|/Game/VRTemplate/Blueprints/VRGameMode.VRGameMode_C|GetQuest _asvrgame_mode)
      (:%20%20
        (Default|CheckQuest _asvrgame_mode)
        (bind _returnvalue (UserInterface|CreateWidget "/Game/VR/blueprints/QuestScreen.QuestScreen_C"))
        (UserInterface|Viewport|AddtoViewport _returnvalue 0)
        (Utilities|FlowControl|Delay 3.0)
        (Default|PlayEnd _returnvalue)
        (Utilities|FlowControl|Delay 1.0)
        (Widget|RemovefromParent _returnvalue)))))

(event Custom|Play%20sound
  (if (Variables|Default|GetCan%20play%20sound)
    (Variables|Default|SetCan%20play%20sound false)
    (Audio|PlaySound2D (Variables|Default|GetSound) 0.5 1.0 0.0 0 0)
    (Utilities|FlowControl|Delay (Variables|Default|Getsound%20delay))
    (Variables|Default|SetCan%20play%20sound true)))

(event EventBeginPlay)

(event EventTick
  (params (DeltaSeconds :type Float%20%28single-precision%29))
  (if (Variables|Default|GetSwimming)
    (CallFunction|PlaySound)))

(event Input|ActionEvents|InputActionRestart
  (params (Key :type Key%20Structure :default "None"))
  (:Pressed
    (Game|OpenLevel(byObjectReference) "/Game/VRTemplate/Maps/Beach.Beach")))

(fn ConstructionScript)
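; BP_checkpoint is a VR quest checkpoint that advances the quest when the player reaches it.
; Box overlap by the player character or the VRPawn found at BeginPlay increments Quest on VRGameMode, calls CheckQuest and destroys the checkpoint.
; Every Tick it searches for VRPawns again, turning its text label toward them and scaling it up with distance so it stays readable from afar.
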(event OnComponentBeginOverlap(box_0)
  (params (OverlappedComponent :type Primitive%20Component%20Object%20Reference) (OtherActor :type Actor%20Object%20Reference) (OtherComp :type Primitive%20Component%20Object%20Reference) (OtherBodyIndex :type Integer) (bFromSweep :type Boolean) (SweepResult :type Hit%20Result%20Structure%20%28by%20ref%29))
  (if (or (== OtherActor (Game|GetPlayerCharacter 0)) (== OtherActor (Variables|Default|GetVr%20pawn)))
    (bind _asvrgame_mode (Utilities|Casting|CastToVRGameMode (Game|GetGameMode)))
    (Math|Integer|IncrementInt (Variables|/Game/VRTemplate/Blueprints/VRGameMode.VRGameMode_C|GetQuest _asvrgame_mode)
      (:%20%20
        (Default|CheckQuest _asvrgame_mode)
        (Actor|DestroyActor)))))

(event EventBeginPlay
  (bind _outactors (Actor|GetAllActorsOfClass "/Game/VRTemplate/Blueprints/VRPawn.VRPawn_C"))
  (for _array_element _outactors
    (Variables|Default|SetVr%20pawn _array_element)))

(event Collision|EventActorBeginOverlap
  (params (OtherActor :type Actor%20Object%20Reference)))

(event EventTick
  (params (DeltaSeconds :type Float%20%28single-precision%29))
  (bind _textrender (Variables|Default|GetTextRender))
  (bind _returnvalue (Transformation|GetWorldLocation _textrender))
  (bind _outactors (Actor|GetAllActorsOfClass "/Game/VRTemplate/Blueprints/VRPawn.VRPawn_C"))
  (for _array_element _outactors
    (Transformation|SetWorldRotation _textrender (Math|Interpolation|RInterpTo (Transformation|GetWorldRotation _textrender) (Math|Rotator|FindLookatRotation _returnvalue (Transformation|GetActorLocation _array_element)) (Utilities|Time|GetWorldDeltaSeconds) 0.0) false false)
    (Transformation|SetWorldScale3D _textrender (Math|Vector|Lerp(Vector) "1.000000,1.000000,1.000000" "30.000000,30.000000,30.000000" (Math|Float|MapRangeClamped (Math|Vector|Distance(Vector) _returnvalue (Transformation|GetActorLocation _array_element)) 5e+02 3e+03 0.0 1.0)))))

(fn ConstructionScript)